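; MyGameCharacter is a player character Blueprint that handles basic movement, camera look and jumping from input mappings.
; Axis inputs drive forward and strafe movement along the actor's forward and right vectors, and feed controller yaw and pitch for looking.
; Pressing Jump copies the JumpHeight variable into JumpMaxHoldTime before jumping, so that variable sets hold duration, and releasing stops the jump.
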(event Input|ActionEvents|InputActionJump
  (params (Key :type Key%20Structure))
  (:Pressed
    (Variables|Default|SetJumpMaxHoldTime (Variables|Default|GetJump%20Height))
    (Character|Jump))
  (:Released
    (Character|StopJumping)))

(event Input|AxisEvents|InputAxisFront_Backward
  (params (AxisValue :type Float%20%28single-precision%29))
  ;[1 1 1] Move
  (Pawn|Input|AddMovementInput (Transformation|GetActorForwardVector) AxisValue false))

(event Input|AxisEvents|InputAxisStrafing
  (params (AxisValue :type Float%20%28single-precision%29))
  ;[1 1 1] Move
  (Pawn|Input|AddMovementInput (Transformation|GetActorRightVector) AxisValue false))

(event Input|AxisEvents|InputAxisRotate
  (params (AxisValue :type Float%20%28single-precision%29))
  ;[1 1 1] Camera Movement
  (Pawn|Input|AddControllerYawInput AxisValue))

(event Input|AxisEvents|InputAxisUpDown
  (params (AxisValue :type Float%20%28single-precision%29))
  ;[1 1 1] Camera Movement
  (Pawn|Input|AddControllerPitchInput AxisValue))

(fn ConstructionScript)